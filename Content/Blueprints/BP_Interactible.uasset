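; BP_Interactible is an interactable actor that the player can activate from within a trigger area.
; BoxTrigger overlap events set PlayInRange when the player's BP_ThirdPersonCharacter enters or leaves.
; The IA_OpenDoor input calls Interact, which sets Interacted only while the player is in range.
; Active returns true until that interaction happens, and nothing here resets it.
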(event `self.Box Trigger.OnComponentBeginOverlap`
  (params (OverlappedComponent :type "PrimitiveComponent Object Reference") (OtherActor :type "Actor Object Reference") (OtherComp :type "PrimitiveComponent Object Reference") (OtherBodyIndex :type Integer) (bFromSweep :type Boolean) (SweepResult :type "HitResult Structure (by ref)"))
  ; Trigger
  (bind _asbp_third_person_character (cast `/Game/ThirdPerson/Blueprints/BP_ThirdPersonCharacter` (`GameplayStatics.GetPlayerPawn` 0)))
  (if (== _asbp_third_person_character OtherActor)
    (set `self.PlayInRange` true)))

(event `self.Box Trigger.OnComponentEndOverlap`
  (params (OverlappedComponent :type "PrimitiveComponent Object Reference") (OtherActor :type "Actor Object Reference") (OtherComp :type "PrimitiveComponent Object Reference") (OtherBodyIndex :type Integer))
  ; Trigger
  (bind _asbp_third_person_character (cast `/Game/ThirdPerson/Blueprints/BP_ThirdPersonCharacter` (`GameplayStatics.GetPlayerPawn` 0)))
  (if (== _asbp_third_person_character OtherActor)
    (set `self.PlayInRange` false)))

(event `Interact`
  (if (`self.PlayInRange`)
    (set `self.Interacted` true)))

(event `EnhancedInput|/Game/Input/IA_OpenDoor`
  (params (ActionValue :type Boolean) (ElapsedSeconds :type "Float (double-precision)") (TriggeredSeconds :type "Float (double-precision)") (InputAction :type "InputAction Object Reference" :default "/Game/Input/IA_OpenDoor.IA_OpenDoor"))
  (:`Triggered`
    (`self.Interact`)))

(fn `Active`
  (returns (ReturnValue :type Boolean))
  (return (not (`self.Interacted`))))

(fn `UserConstructionScript`)