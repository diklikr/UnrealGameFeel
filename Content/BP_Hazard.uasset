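; BP_Hazard is a hazard actor that periodically switches between active and inactive and hurts characters that touch it while active.
; From BeginPlay, the TimeDelay event calls itself after each delay, flipping HazardActive and swapping the mesh material between Rojo and Cafe to show the state.
; Damage applies to a BP_BaseCharacter only when its overlap begins during the active phase.
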(event `self.ReceiveBeginPlay`
  (`self.TimeDelay`))

(event `self.ReceiveActorBeginOverlap`
  (params (OtherActor :type "Actor Object Reference"))
  (if (`self.HazardActive`)
    (bind _asbp_base_character (cast `/Game/ThirdPerson/Blueprints/BP_BaseCharacter` OtherActor))
    (`/Game/ThirdPerson/Blueprints/BP_BaseCharacter.TakeDamage` _asbp_base_character 1)))

(event `TimeDelay`
  (bind _mesh (`self.Mesh`))
  (`KismetSystemLibrary.Delay` (`self.Delay`))
  (bind _output_get (set `self.HazardActive` (not (`self.HazardActive`))))
  (if _output_get
    (`PrimitiveComponent.SetMaterial` _mesh 0 (`self.Rojo`))
    (else
      (`PrimitiveComponent.SetMaterial` _mesh 0 (`self.Cafe`))))
  (`self.TimeDelay`))

(fn `UserConstructionScript`)